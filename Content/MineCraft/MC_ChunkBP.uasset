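; Minecraft-style terrain chunk actor that builds a block of voxels in its construction script.
; Initialize creates one instanced static mesh component per block material, using a shared cube mesh.
; Nested XYZ loops offset column heights with 2D simplex noise sampled at world coordinates derived from actor location.
; 3D simplex noise carves caves with a separate surface-layer cutoff, and remaining voxels get a material by height.
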(event EventBeginPlay)

(fn ConstructionScript
  (bind _returnvalue (Transformation|GetActorLocation))
  (bind _num_2n_1_ (Variables|Default|GetNum%282n+1%29))
  (bind _voxelsize (Variables|Default|GetVoxelSize))
  (bind _num_2n_1__2 (Variables|Default|GetNum%282n+1%29))
  (bind _depth_2n_1_ (Variables|Default|GetDepth%282n+1%29))
  (bind _voxelsize_2 (Variables|Default|GetVoxelSize))
  (bind _3dnoisedensity (Variables|Default|Get3dNoiseDensity))
  (bind _returnvalue_2 (/ _returnvalue _voxelsize))
  (bind (_x _y _z) (Math|Vector|BreakVector _returnvalue_2))
  (CallFunction|Initialize)
  ;[0.15 0.15 0.15 0.5] Loops
  (for _index (range (* _num_2n_1_ -1) _num_2n_1_) ; X
    (Variables|Default|SetLocalVoxelPosX _index)
    (for _index_2 (range (* _num_2n_1__2 -1) _num_2n_1__2) ; Y
      (Variables|Default|SetLocalVoxelPosY _index_2)
      (for _index_3 (range (* _depth_2n_1_ -1) _depth_2n_1_) ; Z
        (Variables|Default|SetLocalVoxelPosZ _index_3)
        ;[0.15 0.15 0.15 0.5] Set Voxel Coordinates(PreNoise)
        (Variables|Default|SetWorldVoxelPosX (+ (Variables|Default|GetLocalVoxelPosX) (Math|Float|Floor _x)))
        (Variables|Default|SetWorldVoxelPosY (+ (Variables|Default|GetLocalVoxelPosY) (Math|Float|Floor _y)))
        (Variables|Default|SetWorldVoxelPosZ-PreNoise (+ (Variables|Default|GetLocalVoxelPosZ) (Math|Float|Floor _z)))
        ;[0.15 0.15 0.15 0.5] Calculate 2D surface Noise
        (bind _returnvalue_3 (Class|SimplexNoiseBPLibrary|SimplexNoise2D (* (Variables|Default|GetWorldVoxelPosX) _voxelsize_2) (* (Variables|Default|GetWorldVoxelPosY) _voxelsize_2) (Variables|Default|GetNoiseDensity)))
        (Variables|Default|SetWorldVoxelPosZ-PostNoise (- (Math|Float|Floor (* (Variables|Default|GetNoiseScale) _returnvalue_3)) (Variables|Default|GetLocalVoxelPosZ)))
        ;[0.15 0.15 0.15 0.5] Apply 3d Noise for Caves
        (if (>= (* (Variables|Default|GetLocalVoxelPosZ) -1) (- (Variables|Default|GetDepth%282n+1%29) 0)) ; Is this the Surface?
          (bind _shouldcutoff_ (CallFunction|Apply3dNoise (Variables|Default|Get3dNoiseCutoffAtSurface) _3dnoisedensity))
          (if (not _shouldcutoff_) ; Is noise LESS than the threshold?
            ;[0.15 0.15 0.15 0.5] Add ISM type depending on Block height
            (if (> (Variables|Default|GetWorldVoxelPosZ-PostNoise) 0) :!label _label
              (CallFunction|AddVoxelInstanceOfTypeUsingWorldPos (Utilities|Array|Get(acopy) (Variables|Default|GetISMs) 2)) ; Grass
              (elif (< (Variables|Default|GetWorldVoxelPosZ-PostNoise) -3)
                (CallFunction|AddVoxelInstanceOfTypeUsingWorldPos (Utilities|Array|Get(acopy) (Variables|Default|GetISMs))) ; Grass
                (else
                  (CallFunction|AddVoxelInstanceOfTypeUsingWorldPos (Utilities|Array|Get(acopy) (Variables|Default|GetISMs) 1)) ; Dirt
                ))))
          (else
            (bind _shouldcutoff__2 (CallFunction|Apply3dNoise (Variables|Default|Get3dNoiseCutoffBelowSurface) _3dnoisedensity))
            (if (not _shouldcutoff__2) ; Is noise LESS than the threshold?
              (goto _label))))))))

(fn Initialize
  (for _array_element (Variables|Default|GetBlockMaterialInstanceTypes)
    (bind _returnvalue (AddComponent|AddInstancedStaticMeshComponent false))
    (Utilities|Array|Add (Variables|Default|GetISMs) _returnvalue)
    (Components|StaticMesh|SetStaticMesh _returnvalue "/Game/LevelPrototyping/Meshes/SM_Cube.SM_Cube")
    (Rendering|Material|SetMaterial _returnvalue 0 _array_element)))

(fn AddVoxelInstanceOfTypeUsingWorldPos
  (params (ISMToAdd :type Instanced%20Static%20Mesh%20Component%20Object%20Reference))
  (Components|InstancedStaticMesh|AddInstance ISMToAdd (Math|Transform|MakeTransform (Math|Vector|MakeVector (* (Variables|Default|GetLocalVoxelPosX) (Variables|Default|GetVoxelSize)) (* (Variables|Default|GetLocalVoxelPosY) (Variables|Default|GetVoxelSize)) (* (Variables|Default|GetWorldVoxelPosZ-PostNoise) (Variables|Default|GetVoxelSize))) "0, 0, 0" (* "1.000000,1.000000,1.000000" (/ (Variables|Default|GetVoxelSize) 1e+02))) false))

(fn Apply3dNoise
  (params (NoiseCutoff :type Float%20%28double-precision%29) (NoiseDensity :type Float%20%28single-precision%29))
  (bind _voxelsize (Variables|Default|GetVoxelSize))
  (bind _returnvalue (Class|SimplexNoiseBPLibrary|SimplexNoise3D (* (Variables|Default|GetWorldVoxelPosX) _voxelsize) (* (Variables|Default|GetWorldVoxelPosY) _voxelsize) (* (Variables|Default|GetWorldVoxelPosZ-PostNoise) _voxelsize) NoiseDensity))
  (return (<= _returnvalue NoiseCutoff)))