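; ISM_Block is a block component for a Minecraft-style game, apparently an instanced static mesh, that sets up its own material from a data asset.
; On BeginPlay it synchronously loads the asset and continues only if it casts to DA_Blocks.
; It creates a dynamic material instance from a transparent or bedrock base according to the block's transparency flag.
; The block data sets that instance's parameters before it is applied to slot zero.
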(event EventBeginPlay
  (bind _returnvalue (Utilities|LoadAssetBlocking (Variables|Default|GetDataAsset)))
  (bind _asda_base (Utilities|Casting|CastToDA_Base _returnvalue))
  (CallFunction|SetupMaterial _asda_base))

(fn SetupMaterial
  (params (InputPin :type DA%20Base%20Object%20Reference))
  (bind _asda_blocks (Utilities|Casting|CastToDA_Blocks InputPin))
  (bind _output_get (Variables|Default|SetLoadedBlock _asda_blocks))
  (bind _returnvalue (Rendering|Material|CreateDynamicMaterialInstance 0 (select (Variables|/Game/MineCraft/DataAssets/BaseClass/DA_Blocks.DA_Blocks_C|GetIsTransparent _output_get) "/Game/MineCraft/Materials/M_Transparent.M_Transparent" "/Game/MineCraft/Materials/MI_Bedrock.MI_Bedrock") "None" :!class /Script/Engine.PrimitiveComponent))
  (Default|SetMaterialParameters (Variables|Default|GetLoadedBlock) _returnvalue)
  (Rendering|Material|SetMaterial 0 _returnvalue))