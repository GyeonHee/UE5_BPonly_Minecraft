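; BP_TerrainGenerator is a test actor that generates a Perlin-noise block terrain chunk at BeginPlay.
; It loops over a ChunkSize grid, sampling FastNoiseWrapper at scaled positions to derive each column's height from HeightScale and BaseHeight.
; Each column adds BlockISM instances, placing the unscaled height index on Y and the noise-space coordinate NoiseZ on Z.
; Debug prints show noise coordinates and computed heights.
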(event EventBeginPlay
  (bind _returnvalue (Game|ConstructObjectfromClass "/Script/FastNoiseGenerator.FastNoiseWrapper"))
  (Class|FastNoiseWrapper|SetupFastNoise _returnvalue "Perlin" 1337 0.5 "Quintic" "FBM" 5 2.0 0.5 0.45 "Euclidean" "CellValue")
  (Variables|Default|SetNoiseGenerator _returnvalue)
  (for _index (range 0 (Variables|Default|GetChunkSize))
    (bind _output_get (Variables|Default|SetCurrentX (* (Math|Conversions|ToFloat(Integer) _index) (Variables|Default|GetVoxelSize))))
    (for _index_2 (range 0 (Variables|Default|GetChunkSize))
      (bind _output_get_2 (Variables|Default|SetCurrentZ (* (Math|Conversions|ToFloat(Integer) _index_2) (Variables|Default|GetVoxelSize))))
      (bind _output_get_3 (Variables|Default|SetNoiseX (/ _output_get (Variables|Default|GetNoiseScale))))
      (Development|PrintString (Utilities|String|ToString(Float) _output_get_3) true true "(R=1.000000,G=0.000000,B=0.000000,A=1.000000)")
      (bind _output_get_4 (Variables|Default|SetNoiseZ (/ _output_get_2 (Variables|Default|GetNoiseScale))))
      (Development|PrintString (Utilities|String|ToString(Float) _output_get_4) true true "(R=0.000000,G=0.000000,B=1.000000,A=1.000000)")
      (bind _output_get_5 (Variables|Default|SetSurfaceHeight (+ (* (Class|FastNoiseWrapper|GetNoise2D (Variables|Default|GetNoiseGenerator) _output_get_3 _output_get_4) (Variables|Default|GetHeightScale)) (Variables|Default|GetBaseHeight))))
      (Development|PrintString (Utilities|String|ToString(Float) _output_get_5))
      (bind _output_get_6 (Variables|Default|SetMaxHeight (Class|KismetMathLibrary|ToInt64(Float) _output_get_5)))
      (Development|PrintString (Utilities|String|ToString(Integer) _output_get_6))
      (for _index_3 (range 0 (Math|Conversions|ToInteger(Byte) _output_get_6))
        (bind _output_get_7 (Variables|Default|SetCurrentY (Math|Conversions|ToFloat(Integer) _index_3)))
        (Components|InstancedStaticMesh|AddInstance (Variables|Default|GetBlockISM) (Math|Transform|MakeTransform (Math|Vector|MakeVector _output_get _output_get_7 _output_get_4)) false)))))

(fn ConstructionScript)